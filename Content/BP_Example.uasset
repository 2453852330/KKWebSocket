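; BP_Example is a skeleton example of a KK WebSocket client, with no working behavior as wired.
; A chained sequence creates a socket, binds closed, connected, error, message, message-sent and raw-message events, then connects and sends a message.
; The URL and message are blank, every handler is empty, and neither that chain nor the separate close call is triggered by any event.
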(event `CustomEvent_3`
  (params (Message :type String)))

(event `CustomEvent_5`
  (params (Data :type "Array of Byte (by ref)") (BytesRemaining :type Integer)))

(event `CustomEvent_1`)

(event `CustomEvent_2`
  (params (Message :type String)))

(event `CustomEvent_4`
  (params (Message :type String)))

(event `CustomEvent_0`
  (params (StatusCode :type Integer) (Reason :type String) (bWasClean :type Boolean)))

(fn `UserConstructionScript`)